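; Player pawn for a rail shooter that tracks health and ammo and forwards left mouse clicks to the game mode.
; BeginPlay fills both stats and takes the HUD widget from the game mode to show ammo.
; PlayerHit recolors and dims three health icons, showing a lose screen and quitting as a placeholder when health drops to 1.
; PlayerHeal restores full health and turns the icons green, without resetting opacity.
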(event Custom|PlayerHit
  (bind _ui_widget_ref (Variables|Default|GetUi%20Widget%20Ref))
  (bind _health2 (Variables|/Game/JamAssets/Player/PlayerUI_BP.PlayerUI_BP_C|GetHealth2 _ui_widget_ref))
  (bind _health1 (Variables|/Game/JamAssets/Player/PlayerUI_BP.PlayerUI_BP_C|GetHealth1 _ui_widget_ref))
  ;[1 1 1] Player Damage
  (if (> (- (Variables|Default|GetPlayerHealth) 1) 0)
    (Variables|Default|SetPlayerHealth (- (Variables|Default|GetPlayerHealth) 1))
    (else
      (Variables|Default|SetPlayerHealth 0)))
  ;[1 1 1] Update Player UI Health Icons
  (switch int (- (Variables|Default|GetPlayerHealth) 1)
    (:0
      (Class|Image|SetOpacity _health1 0.2)
      (bind _returnvalue (UserInterface|CreateWidget "/Game/JamAssets/Player/RailShooter_LoseScreen.RailShooter_LoseScreen_C" (Game|GetPlayerController 0)))
      (UserInterface|Viewport|AddtoViewport _returnvalue 0)
      (Utilities|FlowControl|Delay 0.2)
      ;;[1 0 0.01061] PlaceHolder for return to main menu
      (Game|QuitGame 0 "Quit" false))
    (:1
      (Class|Image|SetOpacity _health2 0.2)
      (Appearance|SetColorandOpacity _health1 "(R=0.411458,G=0.000000,B=0.000000,A=1.000000)" :!class /Script/UMG.Image))
    (:2
      (Class|Image|SetOpacity (Variables|/Game/JamAssets/Player/PlayerUI_BP.PlayerUI_BP_C|GetHealth3 _ui_widget_ref) 0.2)
      (Appearance|SetColorandOpacity _health2 "(R=0.760417,G=0.702445,B=0.000000,A=1.000000)" :!class /Script/UMG.Image))))

(event Custom|PlayerHeal
  (bind _maxplayerhealth (Variables|Default|GetMaxPlayerHealth))
  ;[1 1 1] Player healing
  (if (< (Variables|Default|GetPlayerHealth) _maxplayerhealth)
    (Variables|Default|SetPlayerHealth _maxplayerhealth)
    ;[1 1 1] Update Player UI Health Icons
    (Appearance|SetColorandOpacity (Variables|/Game/JamAssets/Player/PlayerUI_BP.PlayerUI_BP_C|GetHealth1 (Variables|Default|GetUi%20Widget%20Ref)) "(R=0.026846,G=0.489583,B=0.041796,A=1.000000)" :!class /Script/UMG.Image)))

(event EventBeginPlay
  ;[1 1 1] Set Initial Health, Ammo, and UI Ammo Text
  (Variables|Default|SetPlayerHealth (Variables|Default|GetMaxPlayerHealth))
  (bind _output_get (Variables|Default|SetAmmo (Variables|Default|GetMaxAmmo)))
  (bind _asrail_shooter_game_mode_bp (Utilities|Casting|CastToRailShooterGameMode_BP (Game|GetGameMode)))
  (bind _output_get_2 (Variables|Default|SetAs%20Rail%20Shooter%20Game%20Mode%20BP _asrail_shooter_game_mode_bp))
  (bind _output_get_3 (Variables|Default|SetUi%20Widget%20Ref (Variables|/Game/JamAssets/RailShooterGameMode_BP.RailShooterGameMode_BP_C|GetUiWidget_Ref _output_get_2)))
  (Rendering|Components|TextRender|SetText (Variables|/Game/JamAssets/Player/PlayerUI_BP.PlayerUI_BP_C|GetAmmoText _output_get_3) (Utilities|Text|ToText(Integer) _output_get)))

(event Input|MouseEvents|LeftMouseButton
  (params (Key :type Key%20Structure :default "None"))
  (:Pressed
    (Default|Clicked (Variables|Default|GetAs%20Rail%20Shooter%20Game%20Mode%20BP))))

(fn ConstructionScript)