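; RetreatExplosion_BP is a player explosion actor, apparently tied to a retreat move, that damages enemies within an expanding box.
; On BeginPlay it spawns a scaled explosion particle at its root and uses a Timeline to grow the Box from near zero to a multiple of its initial scale.
; Any actor that begins overlapping it receives DamageEnemyMessage with the Damage value.
; The graph contains no logic to destroy the actor afterward.
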(event EventBeginPlay
  (bind _scalemultiplyer (Variables|Default|GetScaleMultiplyer))
  (bind _defaultsceneroot (Variables|Default|GetDefaultSceneRoot))
  (bind _returnvalue (Transformation|GetWorldTransform _defaultsceneroot))
  (Effects|SpawnEmitteratLocation "/Game/StarterContent/Particles/P_Explosion.P_Explosion" (.location _returnvalue) (.rotation _returnvalue) (Math|Vector|MakeVector _scalemultiplyer _scalemultiplyer _scalemultiplyer))
  (bind _output_get (Variables|Default|SetCollisionBoxSize (* (Transformation|GetWorldScale (Variables|Default|GetBox)) "20.000000,20.000000,10.000000")))
  (bind _newtrack_0 (Timeline|Timeline_0 Play)
    (:Update
      (Transformation|SetWorldScale3D (Variables|Default|GetBox) (Math|Vector|Lerp(Vector) "0.010000,0.010000,0.010000" _output_get _newtrack_0)))))

(event Collision|EventActorBeginOverlap
  (params (OtherActor :type Actor%20Object%20Reference))
  (Class|InteractionBPI|DamageEnemy(Message) OtherActor (Variables|Default|GetDamage)))

(fn ConstructionScript)