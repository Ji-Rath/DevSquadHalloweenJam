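; Sliding double door Blueprint whose Right and Left components move apart along world X to open and back together to close.
; BeginPlay caches each panel's start location and an end location offset by MoveDistance in opposite X directions.
; Open plays a timeline that lerps both panels between those points, and Close reverses it from the end.
; Movement uses world axes, so it ignores the actor's rotation.
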(event Custom|Close
  (bind _newtrack_0 (Timeline|Timeline_0 ReverseFromEnd)
    (:Update
      (Transformation|SetWorldLocation (Variables|Default|GetRight) (Math|Vector|Lerp(Vector) (Variables|Default|GetRightStartingLoc) (Variables|Default|GetRightEndLoc) _newtrack_0) false false)
      (Transformation|SetWorldLocation (Variables|Default|GetLeft) (Math|Vector|Lerp(Vector) (Variables|Default|GetLeftStartingLoc) (Variables|Default|GetLeftEndLoc) _newtrack_0) false false))))

(event Custom|Open
  (bind _newtrack_0 (Timeline|Timeline_0 PlayFromStart)
    (:Update
      (Transformation|SetWorldLocation (Variables|Default|GetRight) (Math|Vector|Lerp(Vector) (Variables|Default|GetRightStartingLoc) (Variables|Default|GetRightEndLoc) _newtrack_0) false false)
      (Transformation|SetWorldLocation (Variables|Default|GetLeft) (Math|Vector|Lerp(Vector) (Variables|Default|GetLeftStartingLoc) (Variables|Default|GetLeftEndLoc) _newtrack_0) false false))))

(event EventBeginPlay
  (bind _right (Variables|Default|GetRight))
  (bind _left (Variables|Default|GetLeft))
  (bind _returnvalue (Transformation|GetWorldLocation _left))
  (bind _returnvalue_2 (Transformation|GetWorldLocation _right))
  (bind (_x _y _z) (Math|Vector|BreakVector _returnvalue))
  (bind (_x_2 _y_2 _z_2) (Math|Vector|BreakVector _returnvalue_2))
  (Variables|Default|SetRightStartingLoc _returnvalue_2)
  (Variables|Default|SetRightEndLoc (Math|Vector|MakeVector (+ _x_2 (Variables|Default|GetMoveDistance)) _y_2 _z_2))
  (Variables|Default|SetLeftStartingLoc _returnvalue)
  (Variables|Default|SetLeftEndLoc (Math|Vector|MakeVector (- _x (Variables|Default|GetMoveDistance)) _y _z)))

(fn ConstructionScript)