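; Base enemy character with health, randomized walk speed and behavior-tree-driven idle, wander or combat states.
; Behaviors are injected as dynamic subtrees by gameplay tag, and damage switches idle or wandering enemies to the main tree, which focuses the player.
; Lethal damage has a random chance to spawn a drop.
; Attack and death functions fire dispatchers, with death also unpossessing, stopping movement, disabling capsule collision and starting a timer.
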(event Custom|EnemyDamaged
  (params (Damage :type Float%20%28single-precision%29))
  (bind _returnvalue (Transformation|GetActorTransform))
  (Variables|Default|SetCurrentHealth (- (Variables|Default|GetCurrentHealth) Damage))
  (CallFunction|AggroPlayer)
  (if (<= (Variables|Default|GetCurrentHealth) 0.0)
    (if (== (Math|Random|RandomIntegerinRange 0 2) 1)
      (Game|SpawnActorfromClass "/Game/JamAssets/Enemies/Drops_BP.Drops_BP_C" (Math|Transform|MakeTransform (.location _returnvalue) (.rotation _returnvalue)) "Undefined" 0 0))))

(event EventBeginPlay
  (Variables|Default|SetCurrentHealth (Variables|Default|GetMaxHealth))
  (if (Variables|AI|GetbStartIdle)
    _
    (else
      (CallFunction|SetEnemyBehavior (Variables|AI|GetBehaviorTree))))
  (if (Variables|AI|GetbStartWandering)
    (CallFunction|SetEnemyBehavior "/Game/JamAssets/AI/Wander_BT.Wander_BT")
    (Variables|/Script/Engine.CharacterMovementComponent|SetbOrientRotationToMovement (Variables|Character|GetCharacterMovement) true)))

(event Collision|EventActorBeginOverlap
  (params (OtherActor :type Actor%20Object%20Reference)))

(event EventTick
  (params (DeltaSeconds :type Float%20%28single-precision%29)))

(fn ConstructionScript
  (Variables|/Script/Engine.CharacterMovementComponent|SetMaxWalkSpeed (Variables|Character|GetCharacterMovement) (Math|Random|RandomFloatinRange (Variables|AI|GetMinSpeed) (Variables|AI|GetMaxSpeed))) ; Set random move speed
)

(fn Attack
  (Default|CallOnEnemyAttack))

(fn EnemyDead
  (if (not (Variables|Default|GetbDead))
    (Default|CallOnEnemyDead)
    (Pawn|UnPossess (Pawn|GetController))
    (Components|Movement|StopMovementImmediately (Variables|Character|GetCharacterMovement))
    (Utilities|Time|SetTimerbyEvent (EventDispatchers|CreateEvent :!event K2DestroyActor) 5.0)
    (Variables|Default|SetbDead true)
    (Collision|SetCollisionEnabled (Variables|Collision|GetCapsuleComponent) "NoCollision")))

(fn SetEnemyBehavior
  (params (NewBehavior :type Behavior%20Tree%20Object%20Reference))
  (bind _returnvalue (Pawn|GetController))
  (Utilities|IsValid _returnvalue
    (:Is%20Valid
      (Class|BehaviorTreeComponent|SetDynamicSubtree (Actor|GetComponentbyClass _returnvalue "/Script/AIModule.BehaviorTreeComponent") "(TagName=\"EnemyBehavior\")" NewBehavior)
      (if (== (Variables|AI|GetBehaviorTree) NewBehavior)
        (bind _asaicontroller (Utilities|Casting|CastToAIController (Pawn|GetController)))
        (AI|SetFocus _asaicontroller (Game|Player|GetPlayerPawn 0))
        (Variables|/Script/Engine.CharacterMovementComponent|SetbOrientRotationToMovement (Variables|Character|GetCharacterMovement) false)))))

(fn AggroPlayer
  (if (or (Variables|AI|GetbStartIdle) (Variables|AI|GetbStartWandering))
    (CallFunction|SetEnemyBehavior (Variables|AI|GetBehaviorTree))))