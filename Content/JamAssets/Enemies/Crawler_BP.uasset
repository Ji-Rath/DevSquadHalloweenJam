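; Crawler enemy that randomly starts on the ground or hanging from the ceiling, with an attached breathing sound at a random start offset.
; SetOrientation capsule-traces upward and moves only the mesh to the hit surface, aligned to its normal, while the actor stays below.
; Attacking from the roof teleports the actor up by the mesh offset and restores the mesh transform, a workaround for a smooth fall.
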(event EventBeginPlay
  (|CallParentFunction)
  (Variables|Default|SetDefaultMeshLocation (Transformation|GetRelativeTransform (Variables|Character|GetMesh)))
  (CallFunction|SetOrientation (Math|Random|RandomBool))
  (Audio|SpawnSoundAttached "/Game/JamAssets/Enemies/Sound/Breathing_Cue.Breathing_Cue" (Variables|Transformation|GetRootComponent) "None" "0, 0, 0" "0, 0, 0" "KeepRelativeOffset" true 1.0 1.0 (Math|Random|RandomFloatinRange 0.0 1.0) 0 0))

(event EventTick
  (params (DeltaSeconds :type Float%20%28single-precision%29))
  (|CallParentFunction DeltaSeconds))

(fn ConstructionScript
  (|CallParentFunction))

(fn SetOrientation
  (params (bOnRoof :type Boolean))
  (bind _returnvalue (Transformation|GetActorLocation))
  (bind _mesh (Variables|Character|GetMesh))
  (bind _defaultmeshlocation (Variables|Default|GetDefaultMeshLocation))
  (bind _mesh_2 (Variables|Character|GetMesh))
  (if (Math|Boolean|NotEqual(Boolean) bOnRoof (Variables|Default|GetIsOnRoof))
    (bind _output_get (Variables|Default|SetIsOnRoof bOnRoof))
    (if _output_get
      (bind (_outhit _returnvalue_2) (Collision|CapsuleTraceByChannel _returnvalue (+ _returnvalue (* (Transformation|GetActorUpVector) 1e+03)) 2e+01 88.0 "TraceTypeQuery1" false 0 "None")) ; Trace to find spot to place mesh on roof
      (if _returnvalue_2
        (Transformation|SetRelativeLocation _mesh_2 (- (- (.Location (Collision|BreakHitResult _outhit)) (Transformation|GetActorLocation)) "0, 0,-88.000000") false false)
        (Transformation|SetRelativeRotation _mesh_2 (Math|Rotator|MakeRotfromZ (.ImpactNormal (Collision|BreakHitResult _outhit))) false false)
        (else
          (Variables|Default|SetIsOnRoof false)))
      (else
        (Transformation|Teleport (+ (Transformation|GetActorLocation) (.location (Transformation|GetRelativeTransform (Variables|Character|GetMesh)))) (Transformation|GetActorRotation)) ; Janky solution to have enemy smoothly fall to the ground
        (Transformation|SetRelativeLocation _mesh (.location _defaultmeshlocation) false false)
        (Transformation|SetRelativeRotation _mesh (.rotation _defaultmeshlocation) false false)))))

(fn Attack
  (|CallParentFunction)
  (if (Variables|Default|GetIsOnRoof)
    (CallFunction|SetOrientation false)))